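; Shield generator hazard with two beam collision volumes that kill the first-person character unless they are blocking with a shield.
; A successful block in either beam hides the GeneratorShield component and disables its collision.
; When the character leaves either beam, the shield's visibility and collision are restored, without checking the other beam.
; Both beams run identical overlap logic with debug prints.
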(event OnComponentBeginOverlap(BeamCollison2)
  (params (OtherActor :type Actor%20Object%20Reference) (OtherComp :type Primitive%20Component%20Object%20Reference) (OtherBodyIndex :type Integer) (bFromSweep :type Boolean) (SweepResult :type Hit%20Result%20Structure%20%28by%20ref%29))
  (bind _generator_shield (Variables|Default|GetGenerator_Shield))
  (bind _asfirst_person_character (Utilities|Casting|CastToFirstPersonCharacter OtherActor))
  (if (and (Variables|/Game/Blueprints/FirstPersonBP/Blueprints/FirstPersonCharacter.FirstPersonCharacter_C|GetIsShieldBlock _asfirst_person_character) (Variables|/Game/Blueprints/FirstPersonBP/Blueprints/FirstPersonCharacter.FirstPersonCharacter_C|GetIsShield _asfirst_person_character))
    (Rendering|SetVisibility _generator_shield false false)
    (Collision|SetCollisionEnabled _generator_shield "NoCollision")
    (Development|PrintString "Collision")
    (else
      (Default|CharDeath _asfirst_person_character))))

(event OnComponentEndOverlap(BeamCollison2)
  (params (OtherActor :type Actor%20Object%20Reference) (OtherComp :type Primitive%20Component%20Object%20Reference) (OtherBodyIndex :type Integer))
  (bind _generator_shield (Variables|Default|GetGenerator_Shield))
  (Utilities|Casting|CastToFirstPersonCharacter OtherActor)
  (Rendering|SetVisibility _generator_shield true false)
  (Collision|SetCollisionEnabled _generator_shield "QueryAndPhysics")
  (Development|PrintString "Collision End"))

(event OnComponentBeginOverlap(BeamCollison)
  (params (OtherActor :type Actor%20Object%20Reference) (OtherComp :type Primitive%20Component%20Object%20Reference) (OtherBodyIndex :type Integer) (bFromSweep :type Boolean) (SweepResult :type Hit%20Result%20Structure%20%28by%20ref%29))
  (bind _generator_shield (Variables|Default|GetGenerator_Shield))
  (bind _asfirst_person_character (Utilities|Casting|CastToFirstPersonCharacter OtherActor))
  (if (and (Variables|/Game/Blueprints/FirstPersonBP/Blueprints/FirstPersonCharacter.FirstPersonCharacter_C|GetIsShieldBlock _asfirst_person_character) (Variables|/Game/Blueprints/FirstPersonBP/Blueprints/FirstPersonCharacter.FirstPersonCharacter_C|GetIsShield _asfirst_person_character))
    (Rendering|SetVisibility _generator_shield false false)
    (Collision|SetCollisionEnabled _generator_shield "NoCollision")
    (Development|PrintString "Collision")
    (else
      (Default|CharDeath _asfirst_person_character))))

(event OnComponentEndOverlap(BeamCollison)
  (params (OtherActor :type Actor%20Object%20Reference) (OtherComp :type Primitive%20Component%20Object%20Reference) (OtherBodyIndex :type Integer))
  (bind _generator_shield (Variables|Default|GetGenerator_Shield))
  (Utilities|Casting|CastToFirstPersonCharacter OtherActor)
  (Rendering|SetVisibility _generator_shield true false)
  (Collision|SetCollisionEnabled _generator_shield "QueryAndPhysics")
  (Development|PrintString "Collision End"))

(event EventBeginPlay)

(event EventActorBeginOverlap
  (params (OtherActor :type Actor%20Object%20Reference)))

(event EventTick
  (params (DeltaSeconds :type Float%20%28single-precision%29)))

(fn ConstructionScript)