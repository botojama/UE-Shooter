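; Multiplayer game mode that handles player login, team-based respawning and kill notifications.
; PostLogin assigns each player a number, notifies their controller and sorts tagged PlayerStarts into arrays read only by disconnected old respawn logic.
; RespawnPlayer destroys the current character, then spawns and possesses a default pawn at a random respawn point matching the player's team.
; AddKill broadcasts names and team colors to every PlayerState, crediting the victim when no killer is valid.
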(event Custom|RespawnPlayerEvent
  (params (PlayerController :type Player%20Controller%20Object%20Reference))
  ;[1 1 1] Respawn
  (CallFunction|RespawnPlayer PlayerController))

(event EventPostLogin
  (params (NewPlayer :type Player%20Controller%20Object%20Reference))
  ;[1 1 1] Post Login
  (Networking|SwitchHasAuthority
    (:Authority
      (bind _outactors (Actor|GetAllActorsOfClass "/Script/Engine.PlayerStart"))
      (for _array_element _outactors
        (if (Utilities|Name|Equal(Name) (Variables|/Script/Engine.PlayerStart|GetPlayerStartTag _array_element) "Player1")
          (Utilities|Array|AddUnique (Variables|Default|GetPlayer1) _array_element)
          (else
            (Utilities|Array|AddUnique (Variables|Default|GetPlayer2) _array_element))))
      (bind _asps_mpplayer_state (Utilities|Casting|CastToPS_MPPlayerState (Variables|/Script/Engine.Controller|GetPlayerState NewPlayer)))
      (Variables|/Game/Blueprints/Multiplayer/PS_MPPlayerState.PS_MPPlayerState_C|SetPlayerNumber _asps_mpplayer_state (Utilities|Array|Length (Variables|/Script/Engine.GameState|GetPlayerArray (Game|GetGameState))))
      (bind _aspc_mpplayer_controller (Utilities|Casting|CastToPC_MPPlayerController NewPlayer))
      (Default|ClientPostLogin _aspc_mpplayer_controller))))

(fn ConstructionScript)

(fn SendKillNotification
  (params (Killer :type PS%20MP%20Player%20State%20Object%20Reference) (Victim :type PS%20MP%20Player%20State%20Object%20Reference))
  (bind _returnvalue (Game|GetGameState))
  (bind _teamnumber (Variables|/Game/Blueprints/Multiplayer/PS_MPPlayerState.PS_MPPlayerState_C|GetTeamNumber Killer))
  (bind _teamnumber_2 (Variables|/Game/Blueprints/Multiplayer/PS_MPPlayerState.PS_MPPlayerState_C|GetTeamNumber Victim))
  (bind _asgs_mpgame_state (Utilities|Casting|CastToGS_MPGameState _returnvalue))
  (bind _teamdata (Variables|/Game/Blueprints/Multiplayer/GS_MPGameState.GS_MPGameState_C|GetTeamData _asgs_mpgame_state))
  (bind _item (Utilities|Array|Get(acopy) _teamdata _teamnumber))
  (bind _item_2 (Utilities|Array|Get(acopy) _teamdata _teamnumber_2))
  (Utilities|FlowControl|Sequence
    (:then_0
      (Utilities|IsValid Killer
        (:Is%20Valid
          (LocalVariables|SetKillerName (Utilities|Text|ToText(String) (Variables|/Script/Engine.PlayerState|GetPlayerName Killer)))
          (Utilities|IsValid _item
            (:Is%20Valid
              (LocalVariables|SetTeamColorKiller (Variables|/Game/Blueprints/Multiplayer/TeamData/BP_TeamsData.BP_TeamsData_C|GetTeamColor _item)))))))
    (:then_1
      (Utilities|IsValid Victim
        (:Is%20Valid
          (LocalVariables|SetVictimName (Utilities|Text|ToText(String) (Variables|/Script/Engine.PlayerState|GetPlayerName Victim)))
          (Utilities|IsValid _item_2
            (:Is%20Valid
              (LocalVariables|SetTeamColorVictim (Variables|/Game/Blueprints/Multiplayer/TeamData/BP_TeamsData.BP_TeamsData_C|GetTeamColor _item_2)))))))
    (:then_2
      (for _array_element (Variables|/Script/Engine.GameState|GetPlayerArray (.AsGS%20MPGame%20State (Utilities|Casting|CastToGS_MPGameState (Game|GetGameState))))
        (bind _asps_mpplayer_state (Utilities|Casting|CastToPS_MPPlayerState _array_element))
        (Default|ReceiveKillNotify _asps_mpplayer_state (LocalVariables|GetKillerName) (LocalVariables|GetVictimName) (LocalVariables|GetTeamColorKiller) (LocalVariables|GetTeamColorVictim))))))

(fn AddKill
  (params (Killer :type Controller%20Object%20Reference) (Victim :type First%20Person%20Character%20Object%20Reference))
  (bind _playerstate (Variables|/Script/Engine.Pawn|GetPlayerState Victim))
  (bind _asps_mpplayer_state (Utilities|Casting|CastToPS_MPPlayerState _playerstate))
  (Utilities|IsValid Killer
    (:Is%20Valid
      (CallFunction|SendKillNotification (.AsPS%20MPPlayer%20State (Utilities|Casting|CastToPS_MPPlayerState (Variables|/Script/Engine.Controller|GetPlayerState Killer))) _asps_mpplayer_state))
    (:Is%20Not%20Valid
      (CallFunction|SendKillNotification _asps_mpplayer_state _asps_mpplayer_state))))

(fn RespawnPlayer
  (params (RespawningController :type Controller%20Object%20Reference))
  (bind _returnvalue (Pawn|GetControlledPawn RespawningController))
  (Utilities|FlowControl|Sequence
    (:then_0
      (Utilities|IsValid _returnvalue
        (:Is%20Valid
          (bind _asfirst_person_character (Utilities|Casting|CastToFirstPersonCharacter _returnvalue))
          (Actor|DestroyActor _asfirst_person_character)
          (Pawn|UnPossess RespawningController))))
    (:then_1
      (bind _returnvalue_2 (Game|SpawnActorfromClass (Variables|Default|GetDefaultPawnClass) (Transformation|GetActorTransform (CallFunction|FindSpawnPoint RespawningController)) "AdjustIfPossibleButAlwaysSpawn" RespawningController 0))
      (Pawn|Possess RespawningController _returnvalue_2))))

(fn FindSpawnPoint
  (params (RespawningControllerIn :type Controller%20Object%20Reference))
  (bind _outputspawnpoints (LocalVariables|GetOutputSpawnPoints))
  (bind _outactors (Actor|GetAllActorsOfClass "/Game/Blueprints/Multiplayer/PS_PlayerRespawn.PS_PlayerRespawn_C"))
  (for _array_element _outactors
    (if (== (Variables|/Game/Blueprints/Multiplayer/PS_PlayerRespawn.PS_PlayerRespawn_C|GetTeamNumber _array_element) (Variables|/Game/Blueprints/Multiplayer/PS_MPPlayerState.PS_MPPlayerState_C|GetTeamNumber (.AsPS%20MPPlayer%20State (Utilities|Casting|CastToPS_MPPlayerState (Variables|/Script/Engine.Controller|GetPlayerState RespawningControllerIn)))))
      (Utilities|Array|AddUnique (LocalVariables|GetOutputSpawnPoints) _array_element)))
  (return (Utilities|Array|Get(acopy) _outputspawnpoints (Math|Random|RandomIntegerinRange 0 (- (Utilities|Array|Length _outputspawnpoints) 1)))))