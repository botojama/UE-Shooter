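; Door shield actor with three check lights that display a target count through materials and light colors.
; BeginPlay hardcodes the count to two, then sets that many lights to red, with the shield turning red only at three and otherwise green.
; TargetCounter increments the count when IsNeutral is true but does not refresh the visuals.
; Debug print chains for each state are left unconnected.
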(event EventBeginPlay
  (Variables|Default|SetTargetCount 2)
  (Utilities|FlowControl|Sequence
    (:then_0
      (if (== (Variables|Default|GetTargetCount) 0)
        (Rendering|Material|SetMaterial (Variables|Default|GetCheckLight_1) 0 "/Game/Assets/Environment/AssetPack_01/Materials/M_Security_Camera_Alarm_Flashing_Inst.M_Security_Camera_Alarm_Flashing_Inst")
        (Rendering|Components|Light|SetLightColor (Variables|Default|GetCheckLight_1_Light) "(R=0.482353,G=1.000000,B=0.647059,A=0.000000)" true)
        (Rendering|Material|SetMaterial (Variables|Default|GetDoor_Shield) 0 "/Game/Assets/Environment/AssetPack_01/Materials/M_Door_Shield_Green.M_Door_Shield_Green" :!label _label)))
    (:then_1
      (if (== (Variables|Default|GetTargetCount) 1)
        (Rendering|Material|SetMaterial (Variables|Default|GetCheckLight_1) 0 "/Game/Assets/Environment/AssetPack_01/Materials/M_Security_Camera_Alarm_Flashing_TeamRed.M_Security_Camera_Alarm_Flashing_TeamRed")
        (Rendering|Components|Light|SetLightColor (Variables|Default|GetCheckLight_1_Light) "(R=1.000000,G=0.019608,B=0.019608,A=1.000000)" true)
        (goto _label)))
    (:then_2
      (if (== (Variables|Default|GetTargetCount) 2)
        (Rendering|Material|SetMaterial (Variables|Default|GetCheckLight_2) 0 "/Game/Assets/Environment/AssetPack_01/Materials/M_Security_Camera_Alarm_Flashing_TeamRed.M_Security_Camera_Alarm_Flashing_TeamRed")
        (Rendering|Components|Light|SetLightColor (Variables|Default|GetCheckLight_1_Light) "(R=1.000000,G=0.019608,B=0.019608,A=1.000000)" true)
        (goto _label)))
    (:then_3
      (if (== (Variables|Default|GetTargetCount) 3)
        (Rendering|Material|SetMaterial (Variables|Default|GetCheckLight_1) 0 "/Game/Assets/Environment/AssetPack_01/Materials/M_Security_Camera_Alarm_Flashing_TeamRed.M_Security_Camera_Alarm_Flashing_TeamRed")
        (Rendering|Components|Light|SetLightColor (Variables|Default|GetCheckLight_1_Light) "(R=1.000000,G=0.019608,B=0.019608,A=1.000000)" true)
        (Rendering|Material|SetMaterial (Variables|Default|GetDoor_Shield) 0 "/Game/Assets/Environment/AssetPack_01/Materials/M_Door_Shield_Red.M_Door_Shield_Red")))))

(fn ConstructionScript)

(fn TargetCounter
  (if (Variables|Default|GetIsNeutral)
    (Variables|Default|SetTargetCount (+ (Variables|Default|GetTargetCount) 1))))