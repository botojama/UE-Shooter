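; Central capture point for a team multiplayer mode that awards score to the team holding it.
; Box overlaps track players inside and start an authority-gated timeline capture, which ends if teams mix or the box empties.
; When the timeline finishes, occupants are flagged as holders and a looping timer adds points in the game state for the first occupant's team.
; Debug prints trace each stage.
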(event OnComponentBeginOverlap(Box)
  (params (OtherActor :type Actor%20Object%20Reference) (OtherComp :type Primitive%20Component%20Object%20Reference) (OtherBodyIndex :type Integer) (bFromSweep :type Boolean) (SweepResult :type Hit%20Result%20Structure%20%28by%20ref%29))
  (bind _enteredplayers (Variables|Default|GetEnteredPlayers))
  (bind _asfirst_person_character (Utilities|Casting|CastToFirstPersonCharacter OtherActor)
    (:then
      (Utilities|Array|AddUnique (Variables|Default|GetEnteredPlayers) _asfirst_person_character)
      (Development|PrintString "player entered" true true "(R=0.094116,G=1.000000,B=0.000000,A=1.000000)")
      (CallFunction|PrintTeamNumber)
      (if (> (Utilities|Array|Length _enteredplayers) 0)
        (if (Variables|Default|GetisCapturing)
          (bind _bissameteam (CallFunction|CheckHoldingTeam _enteredplayers))
          (if (not _bissameteam)
            (CallFunction|ServerEndCapture :!label _label)
            (CallFunction|ServerStopHolding)
            (Development|PrintString "NOT SAME TEAM" true true "(R=1.000000,G=0.078045,B=0.701921,A=1.000000)" 15.0))
          (else
            (CallFunction|ServerStartCapture)))
        (else
          (goto _label))))
    (:CastFailed
      (Development|PrintString "YOU NO PLAYER!"))))

(event OnComponentEndOverlap(Box)
  (params (OtherActor :type Actor%20Object%20Reference) (OtherComp :type Primitive%20Component%20Object%20Reference) (OtherBodyIndex :type Integer))
  (bind _enteredplayers (Variables|Default|GetEnteredPlayers))
  (bind _enteredplayers_2 (Variables|Default|GetEnteredPlayers))
  (bind _asfirst_person_character (Utilities|Casting|CastToFirstPersonCharacter OtherActor)
    (:then
      (for (_array_element _array_index) _enteredplayers
        (if (== _array_element _asfirst_person_character)
          (Variables|/Game/Blueprints/FirstPersonBP/Blueprints/FirstPersonCharacter.FirstPersonCharacter_C|SetisHoldingCentralPoint _array_element false)
          (Utilities|Array|RemoveIndex _enteredplayers _array_index)
          (Development|PrintString "player left point" true true "(R=1.000000,G=0.062643,B=0.000000,A=1.000000)")
          (else
            (Development|PrintString "LOL"))))
      (if (> (Utilities|Array|Length _enteredplayers_2) 0)
        (bind _bissameteam (CallFunction|CheckHoldingTeam _enteredplayers_2))
        (if (not _bissameteam)
          (CallFunction|ServerEndCapture :!label _label)
          (CallFunction|ServerStopHolding))
        (else
          (goto _label))))
    (:CastFailed
      (Development|PrintString "LOL"))))

(event Custom|ServerStartCapture
  (Networking|SwitchHasAuthority
    (:Authority
      (Variables|Default|SetisCapturing true)
      (bind _holdtime (Timeline|Timeline_0 PlayFromStart)
        (:Update
          (bind _output_get (Variables|Default|SetCurrentHoldTime%20 _holdtime))
          (Development|PrintString (Utilities|String|ToString(Float) _output_get)))
        (:Finished
          (CallFunction|ServerIsHoldingPoint)
          (Variables|Default|SetisHold true))))))

(event Custom|ServerIsHoldingPoint
  (Networking|SwitchHasAuthority
    (:Authority
      (bind _returnvalue (Utilities|Time|SetTimerbyFunctionName 0 "Holding" 3.0 true))
      (for _array_element (Variables|Default|GetEnteredPlayers)
        (Variables|/Game/Blueprints/FirstPersonBP/Blueprints/FirstPersonCharacter.FirstPersonCharacter_C|SetisHoldingCentralPoint _array_element true)
        (Variables|Default|SetHoldingTeamInt 1)))))

(event Custom|ServerEndCapture
  (Variables|Default|SetisCapturing false)
  (bind _holdtime (Timeline|Timeline_0 Stop)
    (:Update
      (bind _output_get (Variables|Default|SetCurrentHoldTime%20 _holdtime))
      (Development|PrintString (Utilities|String|ToString(Float) _output_get)))
    (:Finished
      (CallFunction|ServerIsHoldingPoint)
      (Variables|Default|SetisHold true))))

(event Custom|ServerStopHolding
  (Class|KismetSystemLibrary|ClearTimerHandle (stale Custom|ServerIsHoldingPoint _returnvalue))
  (Variables|Default|SetisHold false)
  (Variables|Default|SetisCapturing false)
  (Variables|Default|SetHoldingTeamInt 0))

(event EventBeginPlay)

(event EventActorBeginOverlap
  (params (OtherActor :type Actor%20Object%20Reference)))

(event EventTick
  (params (DeltaSeconds :type Float%20%28single-precision%29)))

(fn ConstructionScript)

(fn Holding
  (bind _returnvalue (Game|GetGameState))
  (bind _asgs_mpgame_state (Utilities|Casting|CastToGS_MPGameState _returnvalue))
  (bind _asps_mpplayer_state (Utilities|Casting|CastToPS_MPPlayerState (Variables|/Script/Engine.Pawn|GetPlayerState (Utilities|Array|Get(acopy) (Variables|Default|GetEnteredPlayers)))))
  (if (== (Variables|/Game/Blueprints/Multiplayer/PS_MPPlayerState.PS_MPPlayerState_C|GetTeamNumber _asps_mpplayer_state) 0)
    (Variables|/Game/Blueprints/Multiplayer/GS_MPGameState.GS_MPGameState_C|SetScoreRed _asgs_mpgame_state (+ (Variables|/Game/Blueprints/Multiplayer/GS_MPGameState.GS_MPGameState_C|GetScoreRed _asgs_mpgame_state) 5))
    (Development|PrintString (Utilities|String|Append "Team Red capturing: " (Utilities|String|ToString(Integer) (Variables|/Game/Blueprints/Multiplayer/GS_MPGameState.GS_MPGameState_C|GetScoreRed _asgs_mpgame_state))))
    (else
      (Variables|/Game/Blueprints/Multiplayer/GS_MPGameState.GS_MPGameState_C|SetScoreBlue _asgs_mpgame_state (+ (Variables|/Game/Blueprints/Multiplayer/GS_MPGameState.GS_MPGameState_C|GetScoreBlue _asgs_mpgame_state) 5))
      (Development|PrintString (Utilities|String|Append "Team Blue Capturing: " (Utilities|String|ToString(Integer) (Variables|/Game/Blueprints/Multiplayer/GS_MPGameState.GS_MPGameState_C|GetScoreBlue _asgs_mpgame_state)))))))

(fn CheckHoldingTeam
  (params (EnterPlayers :type Array%20of%20First%20Person%20Character%20Object%20References))
  (for _index (range 0 (- (Utilities|Array|Length EnterPlayers) 1))
    (for _index_2 (range 0 (- (Utilities|Array|Length EnterPlayers) 1))
      (if (not (== (Variables|/Game/Blueprints/Multiplayer/PS_MPPlayerState.PS_MPPlayerState_C|GetTeamNumber (.AsPS%20MPPlayer%20State (Utilities|Casting|CastToPS_MPPlayerState (Variables|/Script/Engine.Pawn|GetPlayerState (Utilities|Array|Get(acopy) EnterPlayers _index_2))))) (Variables|/Game/Blueprints/Multiplayer/PS_MPPlayerState.PS_MPPlayerState_C|GetTeamNumber (.AsPS%20MPPlayer%20State (Utilities|Casting|CastToPS_MPPlayerState (Variables|/Script/Engine.Pawn|GetPlayerState (Utilities|Array|Get(acopy) EnterPlayers _index)))))))
        (return false)))
    (Development|PrintString "first loop comlpete" true true "(R=1.000000,G=0.125357,B=0.448484,A=1.000000)" 5.0))
  (Development|PrintString "ran second loop" true true "(R=1.000000,G=0.064425,B=0.227670,A=1.000000)" 5.0)
  (return true))

(fn PrintTeamNumber
  (for (_array_element _array_index) (Variables|Default|GetEnteredPlayers)
    (Development|PrintString (Utilities|String|Append "Player" (Utilities|String|ToString(Integer) _array_index) "Team" (Utilities|String|ToString(Integer) (Variables|/Game/Blueprints/Multiplayer/PS_MPPlayerState.PS_MPPlayerState_C|GetTeamNumber (.AsPS%20MPPlayer%20State (Utilities|Casting|CastToPS_MPPlayerState (Variables|/Script/Engine.Pawn|GetPlayerState _array_element)))))) true true "(R=1.000000,G=0.943857,B=0.259392,A=1.000000)" 1e+01)))