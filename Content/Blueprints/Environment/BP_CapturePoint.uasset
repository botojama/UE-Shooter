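; BP_CapturePoint is an environment actor that lets the player charge energy while inside its trigger.
; Trigger overlap enables and disables input for player 0, and holding C sets the EnergyLoad flag.
; EnergyFill adds a small fixed amount to the FirstPersonCharacter's CurrentEnergy when that flag is set and MaxEnergy passes a threshold.
; Nothing in this Blueprint calls EnergyFill or caps CurrentEnergy.
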(event OnComponentBeginOverlap(Trigger)
  (params (OtherActor :type Actor%20Object%20Reference) (OtherComp :type Primitive%20Component%20Object%20Reference) (OtherBodyIndex :type Integer) (bFromSweep :type Boolean) (SweepResult :type Hit%20Result%20Structure%20%28by%20ref%29))
  (Input|EnableInput (Game|GetPlayerController 0)))

(event OnComponentEndOverlap(Trigger)
  (params (OtherActor :type Actor%20Object%20Reference) (OtherComp :type Primitive%20Component%20Object%20Reference) (OtherBodyIndex :type Integer))
  (Input|DisableInput (Game|GetPlayerController 0)))

(event Input|KeyboardEvents|C
  (params (Key :type Key%20Structure :default "AnyKey"))
  (:Pressed
    (Variables|Default|SetEnergyLoad true))
  (:Released
    (Variables|Default|SetEnergyLoad false)))

(fn ConstructionScript)

(fn EnergyFill
  (bind _asfirst_person_character (Utilities|Casting|CastToFirstPersonCharacter (Game|GetPlayerCharacter 0)))
  (if (and (Variables|Default|GetEnergyLoad) (>= (Variables|/Game/Blueprints/FirstPersonBP/Blueprints/FirstPersonCharacter.FirstPersonCharacter_C|GetMaxEnergy _asfirst_person_character) 99.0))
    (Variables|/Game/Blueprints/FirstPersonBP/Blueprints/FirstPersonCharacter.FirstPersonCharacter_C|SetCurrentEnergy _asfirst_person_character (+ (Variables|/Game/Blueprints/FirstPersonBP/Blueprints/FirstPersonCharacter.FirstPersonCharacter_C|GetCurrentEnergy _asfirst_person_character) 0.1))))