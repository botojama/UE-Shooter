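; GS_MP is a multiplayer Game State that sets up team data when a match begins.
; On BeginPlay it reads the team count from GM_MP and flags the match as a team game when there is more than one.
; For team games it spawns one actor per team from the DefinedTeams classes at a far-off location, owned by itself, and collects them in TeamData.
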(event EventBeginPlay
  (bind _returnvalue (Game|GetGameMode))
  (bind _asgm_mp (Utilities|Casting|CastToGM_MP _returnvalue))
  (bind _numberofteams (Variables|/Game/Multiplayer/Blueprints/GM_MP.GM_MP_C|GetNumberOfTeams _asgm_mp))
  (bind _output_get (Variables|Default|SetbIsTeamGame (> _numberofteams 1)))
  (if _output_get ; Teams?
    (for _index (range 0 (- _numberofteams 1))
      (bind _returnvalue_2 (Game|SpawnActorfromClass (Utilities|Array|Get(acopy) (Variables|Config|Teams|GetDefinedTeams) _index) (Math|Transform|MakeTransform "9999.000000,9999.000000,9999.000000") "AlwaysSpawn" self 0))
      (Utilities|Array|AddUnique (Variables|Info|GetTeamData) _returnvalue_2))))

(fn ConstructionScript)