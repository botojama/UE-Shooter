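; GS_MPGameState is the multiplayer game state, with replication callbacks for red and blue team scores.
; Both score OnRep functions, BeginPlay and the construction script are empty.
; An unconnected graph fragment would spawn an actor per team from DefinedTeams, up to the game mode's NumberOfTeams, far off at a fixed location and collect them in TeamData, but it never runs.
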(event EventBeginPlay)

(fn ConstructionScript)

(fn OnRepScoreRed)

(fn OnRepScoreBlue)