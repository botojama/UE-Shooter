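; BP_Door_Target is a shootable target that continuously slides back and forth along its relative Y axis.
; BeginPlay marks it neutral and starts an endless loop of two timed MoveComponentTo moves.
; A BP_RailgunProjectile hit on Target_Trigger turns the target material and light red and clears IsNeutral.
; TargetCounter increments and prints TargetCount while the target is neutral, but nothing in this Blueprint calls it.
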(event OnComponentHit(Target_Trigger)
  (params (OtherActor :type Actor%20Object%20Reference) (OtherComp :type Primitive%20Component%20Object%20Reference) (NormalImpulse :type Vector :default "0, 0, 0") (Hit :type Hit%20Result%20Structure%20%28by%20ref%29))
  (Utilities|Casting|CastToBP_RailgunProjectile OtherActor)
  (Rendering|Material|SetMaterial (Variables|Default|GetS_Door_Target) 0 "/Game/Assets/Environment/AssetPack_01/Materials/M_Door_Target_Red.M_Door_Target_Red")
  (Rendering|Components|Light|SetLightColor (Variables|Default|GetTarget_Light) "(R=1.000000,G=0.020000,B=0.020000,A=1.000000)" true)
  (Variables|Default|SetIsNeutral false))

(event EventBeginPlay
  (bind _s_door_target (Variables|Default|GetS_Door_Target))
  (Variables|Default|SetIsNeutral true)
  (Components|MoveComponentTo _s_door_target "0,-900.000000, 0" "0, 0, 0" false false 3.0 :!label _label)
  (Components|MoveComponentTo _s_door_target "0,-100.000000, 0" "0, 0, 0" false false 3.0)
  (goto _label))

(fn ConstructionScript)

(fn TargetCounter
  (if (Variables|Default|GetIsNeutral)
    (Variables|Default|SetTargetCount (+ (Variables|Default|GetTargetCount) 1))
    (Development|PrintString (Utilities|String|ToString(Integer) (Variables|Default|GetTargetCount)))))